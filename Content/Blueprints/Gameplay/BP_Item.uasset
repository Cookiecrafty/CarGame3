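; BP_Item is an item pickup that gives a random item type to a BP_CustomArcadeVehicle driving into it.
; On Cube overlap, it acts only if the vehicle's CurrentItemType equals one specific enum value, then sets that to a random entry from ItemTypes.
; PickItem hides the cube and disables its collision, then a timer calls RespawnItem ten seconds later to restore both.
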(event `self.Cube.OnComponentBeginOverlap`
  (params (OverlappedComponent :type "PrimitiveComponent Object Reference") (OtherActor :type "Actor Object Reference") (OtherComp :type "PrimitiveComponent Object Reference") (OtherBodyIndex :type Integer) (bFromSweep :type Boolean) (SweepResult :type "HitResult Structure (by ref)"))
  (bind _asbp_custom_arcade_vehicle (cast `/Game/Blueprints/Cars/CustomArcadeVehicle/BP_CustomArcadeVehicle` OtherActor))
  (if (`|EnumEquality` (`/Game/Blueprints/Cars/CustomArcadeVehicle/BP_CustomArcadeVehicle.currentItemType` _asbp_custom_arcade_vehicle) "NewEnumerator2")
    (`self.PickItem`)
    (set `/Game/Blueprints/Cars/CustomArcadeVehicle/BP_CustomArcadeVehicle.currentItemType` (`KismetArrayLibrary.Array_Random` (`self.itemTypes`)) _asbp_custom_arcade_vehicle)))

(fn `PickItem`
  (bind _cube (`self.Cube`))
  (`PrimitiveComponent.SetCollisionEnabled` _cube "NoCollision")
  (`SceneComponent.SetHiddenInGame` _cube true false)
  (`KismetSystemLibrary.K2_SetTimer` self "RespawnItem" 10.0))

(fn `RespawnItem`
  (bind _cube (`self.Cube`))
  (`PrimitiveComponent.SetCollisionEnabled` _cube "QueryAndPhysics")
  (`SceneComponent.SetHiddenInGame` _cube false false))

(fn `UserConstructionScript`)
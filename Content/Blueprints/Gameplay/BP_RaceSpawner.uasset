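; Race spawner actor that, when its Multi flag is set, spawns vehicles for local multiplayer on BeginPlay.
; It loops over vehicle classes in GI_CustomVehicleGameInstance, creating a local player for each index after the first.
; Each vehicle gets a player ID and numbered Racer name, then is possessed by its controller.
; Vehicles use separate BP_RaceSpawner transforms when enough exist, otherwise all use this spawner's transform.
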(event `self.ReceiveBeginPlay`
  (if (`self.multi`)
    (bind _asgi_custom_vehicle_game_instance (cast `/Game/Blueprints/GI_CustomVehicleGameInstance` (`GameplayStatics.GetGameInstance`)))
    (bind _outactors (`GameplayStatics.GetAllActorsOfClass` "BP_RaceSpawner_C"))
    (bind _vehicles (`/Game/Blueprints/GI_CustomVehicleGameInstance.vehicles` _asgi_custom_vehicle_game_instance))
    (for (_array_element _array_index) _vehicles
      (`KismetSystemLibrary.PrintString` (`KismetSystemLibrary.GetClassDisplayName` _array_element))
      (if (> _array_index 0)
        (`GameplayStatics.CreatePlayer` _array_index))
      (bind _returnvalue (`|SpawnActorFromClass` _array_element (`self.GetTransform` (select `bool` (>= (`KismetArrayLibrary.Array_Length` _outactors) (`KismetArrayLibrary.Array_Length` _vehicles)) :`false` self :`true` (`|GetArrayItem` _outactors _array_index) :!type "Self Object Reference")) "Undefined" "OverrideRootScale" null _array_index (`KismetTextLibrary.Conv_StringToText` (`KismetStringLibrary.Concat_StrStr` "Racer " (`KismetStringLibrary.Conv_IntToString` (+ _array_index 1)))) null))
      (bind _returnvalue_2 (`GameplayStatics.GetPlayerControllerFromID` _array_index))
      (`Controller.UnPossess` _returnvalue_2)
      (`Controller.Possess` _returnvalue_2 _returnvalue))))

(fn `UserConstructionScript`)
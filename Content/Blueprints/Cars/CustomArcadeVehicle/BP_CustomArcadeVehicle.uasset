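; Player- or AI-possessable arcade car pawn driven by forces on a simulated collision body.
; Each tick, four sphere traces apply spring-damper suspension and set grounded state, which gates throttle, steering torque, boost and anti-slide force.
; Custom gravity and center of mass adapt to falling time, while wheel visuals and engine audio follow movement.
; Also handles timed boost items, camera switching, checkpoint reset, per-player HUD and debug drawing.
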(event `InputAction|ToggleDebug`
  (params (Key :type "Key Structure"))
  ;[1 1 1] Debug
  (:`Pressed`
    (`/Engine/EditorBlueprintResources/StandardMacros.FlipFlop`
      (:`A`
        (`self.SetMeshesVisibility` (`self.shouldDisplayMeshesDuringDebug`))
        (`self.StartDebug`)
        (set `self.isDebugModeEnabled` true))
      (:`B`
        (`self.SetMeshesVisibility` true)
        (`self.StopDebug`)
        (set `self.isDebugModeEnabled` false)))))

(event `self.ReceiveBeginPlay`
  ;[1 1 1] Begin Play
  (`|ExecutionSequence`
    (:`then_0`
      (`self.InitializeConfig`))
    (:`then_1`
      (`self.InitializeComponentArrays`))
    (:`then_2`
      (`self.InitializePhysicsConfiguration`))
    (:`then_3`
      (bind (_direction _alpha) (`Timeline|SuspensionInitTimeline` :!via `PlayFromStart`)
        (:`Update`
          (set `self.currentSuspensionStiffness` (`KismetMathLibrary.Lerp` 0.0 (`self.suspensionStiffness`) _alpha))
          (set `self.currentSuspensionDamping` (`KismetMathLibrary.Lerp` 0.0 (`self.suspensionDamping`) _alpha)))))))

(event `InputAction|SwitchCamera`
  (params (Key :type "Key Structure"))
  ;[1 1 1] Switch Camera
  (:`Pressed`
    (`self.EnableIncarView` (not (`self.IsInCar`)))))

(event `self.ReceiveTick`
  (params (DeltaSeconds :type "Float (single-precision)"))
  ;[1 1 1] Tick
  (set `self.deltaSeconds` DeltaSeconds)
  (if (`SceneComponent.IsSimulatingPhysics` (`self.VehicleCollision`) "None")
    (`|ExecutionSequence`
      (:`then_0`
        (`self.GetCurrentMovementValues`))
      (:`then_1`
        (bind _groundwheelscount (`self.ApplySuspensionForces`))
        (`self.HandleFallingTime` _groundwheelscount))
      (:`then_2`
        (`self.UpdateCenterOfMassOffset`))
      (:`then_3`
        (`self.HandleSpeedBoost`))
      (:`then_4`
        (`self.ApplyGravityAndAntiSlidingForces`))
      (:`then_5`
        (`self.UpdateWheelsPosition`)
        (`self.UpdateWheelsRotation`)
        (`self.UpdateWheelsSteering`))
      (:`then_6`
        (`self.UpdateEngineAudio`))
      (:`then_8`
        (`/Engine/EditorBlueprintResources/StandardMacros.Gate` true :!label _label
          (:`Exit`
            (`self.DrawDebugInfo`)))))))

(event `InputAction|UseItem`
  (params (Key :type "Key Structure"))
  ;[1 1 1] Use Item
  (:`Pressed`
    (`self.UseItem`)))

(event `InputAction|ResetCar`
  (params (Key :type "Key Structure"))
  (bind _vehiclecollision (`self.VehicleCollision`))
  ;[1 1 1] Reset Position to Last Checkpoint
  (:`Pressed`
    (if (`self.bCanReset`)
      (set `self.bCanReset` false)
      (`PrimitiveComponent.SetSimulatePhysics` _vehiclecollision false)
      (`self.K2_SetActorTransform` (`self.lastCheckPointPosition`) false true)
      (set `self.IsInCarForced` false)
      (`self.EnableIncarView` (`self.IsInCar`))
      (`TimelineComponent.PlayFromStart` (`self.SuspensionInitTimeline`))
      (`PrimitiveComponent.SetSimulatePhysics` _vehiclecollision true)
      (`KismetSystemLibrary.K2_SetTimer` self "ResetCarCD" 3.0))))

(event `StartDebug`
  ;[1 1 1] Tick
  (goto _label :!via `Open`))

(event `StopDebug`
  ;[1 1 1] Tick
  (goto _label :!via `Close`))

(event `InputAxis|MoveForward`
  (params (AxisValue :type "Float (single-precision)"))
  ;[1 1 1] Throttle
  (bind _output_get (set `self.currentThrottleAxis` AxisValue))
  (if (and (>= (`KismetMathLibrary.Abs` _output_get) 0.1) (<= (`self.currentHorizontalSpeed`) (`self.maxSpeed`)) (`self.isMovingOnGround`))
    (`PrimitiveComponent.AddForce` (`self.VehicleCollision`) (* (`self.GetActorForwardVector`) (* _output_get (`self.acceleration`))) "None" true)))

(event `InputAxis|MoveRight`
  (params (AxisValue :type "Float (single-precision)"))
  ;[1 1 1] Steering
  (bind _output_get (set `self.currentSteeringAxis` AxisValue))
  (if (and (> (`self.currentHorizontalSpeed`) (`self.minSpeedToSteer`)) (>= (`KismetMathLibrary.Abs` _output_get) 0.1) (`self.isMovingOnGround`))
    (`PrimitiveComponent.AddTorqueInRadians` (`self.VehicleCollision`) (* (`self.GetActorUpVector`) (* (`self.steeringTorque`) _output_get (`KismetMathLibrary.SignOfFloat` (`self.currentMovingDirectionFake`)) (select `bool` (`self.isSpeedBoostEnabled`) :`false` 1.0 :`true` 2.0 :!type "Float (single-precision)"))) "None" true)))

(event `self.ReceivePossessed`
  (params (NewController :type "Controller Object Reference"))
  ;[1 1 1] Possess / Unpossess
  (if (not (`.bSuccess` (cast `AIController` NewController :!pure true)))
    (bind _ingamehud (`self.inGameHUD`)
      (:`then`
        (`UserWidget.AddToPlayerScreen` _ingamehud 0))
      (:`else`
        (`self.InitializeHUD`)))))

(event `SelectCarInteraction`
  (bind (_returnvalue_x _returnvalue_y _returnvalue_z) (`KismetMathLibrary.BreakVector` (`self.K2_GetActorLocation`)))
  ;[1 1 1] Select Car Anim
  (`PrimitiveComponent.SetConstraintMode` (`self.VehicleCollision`) "None")
  (bind (_direction _factor) (`Timeline|AnimateSelectCar` :!via `PlayFromStart`)
    (:`Update`
      (`self.K2_SetActorLocation` (`KismetMathLibrary.MakeVector` _returnvalue_x (+ (* _factor 700.0) (.y (.location (`self.lastCheckPointPosition`)))) _returnvalue_z)))))

(event `self.ReceiveUnpossessed`
  (params (OldController :type "Controller Object Reference"))
  ;[1 1 1] Possess / Unpossess
  (if (not (`.bSuccess` (cast `AIController` OldController :!pure true)))
    (bind _ingamehud (`self.inGameHUD`)
      (:`then`
        (`Widget.RemoveFromParent` _ingamehud))
      (:`else`))))

(fn `ApplyGravityAndAntiSlidingForces`
  (`PrimitiveComponent.AddForce` (`self.VehicleCollision`) (* (select `bool` (< (`self.fallingTime`) 0.5) :`false` (0.0 0.0 1.0) :`true` (`self.GetActorUpVector`)) (* (`self.gravity`) -1.0)) "None" true)
  (set `self.currentSlidingSpeed` (`KismetMathLibrary.Dot_VectorVector` (`self.currentHorizontalVelocity`) (`self.GetActorRightVector`)))
  (if (and (`self.isMovingOnGround`) (> (`self.currentHorizontalSpeed`) 10.0))
    (`PrimitiveComponent.AddForce` (`self.VehicleCollision`) (* (`self.GetActorRightVector`) (* (`self.currentSlidingSpeed`) (`self.antiSlideForce`) -1.0)) "None" true)))

(fn `ApplySuspensionForces`
  (returns (groundWheelsCount :type Integer))
  (set `self.groundedWheelsNum` 0)
  (for (_array_element _array_index) (`self.localSuspensionPointsList`)
    (set `self.currentPointRelativeLocation` _array_element)
    (set `self.currentPointIndex` _array_index)
    (set `self.currentPointWorldLocation` (`KismetMathLibrary.TransformLocation` (`self.GetTransform`) (`self.currentPointRelativeLocation`)))
    (bind (_isgroundhit _ratio _applyforcelocation) (`self.PerformSuspensionRaycasts` (`self.currentPointWorldLocation`) (`self.currentPointRelativeLocation`)))
    (if _isgroundhit
      (`/Engine/EditorBlueprintResources/StandardMacros.IncrementInt` (`self.groundedWheelsNum`)
        (:`  `
          _)))
    (set `self.currentSuspensionRatio` _ratio)
    (`PrimitiveComponent.AddForceAtLocation` (`self.VehicleCollision`) (* (`self.GetActorUpVector`) (* (+ (* (`self.suspensionStiffness`) (`self.currentSuspensionRatio`)) (* (`self.suspensionDamping`) (/ (- (`self.currentSuspensionRatio`) (`|GetArrayItem` (`self.lastFrameRatios`) (`self.currentPointIndex`))) (`self.deltaSeconds`)))) (`self.massInKg`) (`self.gravity`))) _applyforcelocation "None")
    (`KismetArrayLibrary.Array_Set` (`self.lastFrameRatios`) (`self.currentPointIndex`) (`self.currentSuspensionRatio`))
    (if (`self.isDebugModeEnabled`)
      (`KismetSystemLibrary.DrawDebugSphere` _applyforcelocation (`self.contactPointSphereRadius`) 12 (`self.contactPointSphereColor`))))
  (return (`self.groundedWheelsNum`)))

(fn `DrawDebugInfo`
  (bind _vehiclecollision (`self.VehicleCollision`))
  (`KismetSystemLibrary.PrintString` (`KismetStringLibrary.Concat_StrStr` "isMovingOnTheGround : " (`KismetStringLibrary.Conv_BoolToString` (`self.isMovingOnGround`))) true true (struct :`R` 0.670833 :`B` 0.014089 :`A` 1.0) 0.0)
  (`KismetSystemLibrary.PrintString` (`KismetStringLibrary.Conv_DoubleToString` (`self.fallingTime`)) true true (struct :`G` 0.5875 :`B` 0.003383 :`A` 1.0) 0.0)
  (`KismetSystemLibrary.DrawDebugSphere` (`PrimitiveComponent.GetCenterOfMass` (`self.VehicleCollision`) "None") (`self.centerOfMassSphereRadius`) 12 (`self.centerOfMassSphereColor`))
  (`KismetSystemLibrary.DrawDebugBox` (`SceneComponent.K2_GetComponentLocation` _vehiclecollision) (`BoxComponent.GetScaledBoxExtent` _vehiclecollision) (`self.collisionBoxColor`) (`SceneComponent.K2_GetComponentRotation` _vehiclecollision) 0.0 (`self.collisionBoxThickness`))
  (for (_array_element _array_index) (`self.wheelSceneList`)
    (bind _output (`|GetArrayItem` (`self.lastFrameRatios`) _array_index))
    (`KismetSystemLibrary.DrawDebugString` (`SceneComponent.K2_GetComponentLocation` _array_element) (`KismetStringLibrary.Concat_StrStr` (`KismetStringLibrary.GetSubstring` (`KismetSystemLibrary.GetObjectName` _array_element) 0 3) ":" (`KismetStringLibrary.GetSubstring` (`KismetStringLibrary.Conv_DoubleToString` _output) 0 4)) null (`KismetMathLibrary.LinearColorLerp` (struct :`G` 1.0 :`A` 1.0) (struct :`R` 1.0 :`A` 1.0) _output))))

(fn `EnableInCarView`
  (params (isInCar :type Boolean))
  (bind _outsidecam (`self.OutsideCam`))
  (bind _insidecam (`self.InsideCam`))
  (set `self.IsInCar` isInCar)
  (if (or (`self.IsInCar`) (`self.IsInCarForced`))
    ;[1 1 1] Activate Internal, Deactivate chase
    (`ActorComponent.Activate` _insidecam false)
    (`ActorComponent.Deactivate` _outsidecam)
    (else
      ;[1 1 1] Deactivate Internal,  Activate chase
      (`ActorComponent.Deactivate` _insidecam)
      (`ActorComponent.Activate` _outsidecam false)))
  (return))

(fn `GetCurrentMovementValues`
  (bind _returnvalue (`self.GetInputAxisValue`))
  (bind _vehiclecollision (`self.VehicleCollision`))
  (bind _returnvalue_2 (`KismetMathLibrary.ProjectVectorOnToPlane` (`SceneComponent.GetComponentVelocity` _vehiclecollision) (`SceneComponent.GetUpVector` _vehiclecollision)))
  (set `self.isMovingOnGround` false)
  (set `self.currentHorizontalVelocity` _returnvalue_2)
  (set `self.currentHorizontalSpeed` (`KismetMathLibrary.VSize` _returnvalue_2))
  (set `self.currentHorizontalMovementDirection` (`KismetMathLibrary.SignOfFloat` (`KismetMathLibrary.Dot_VectorVector` (`KismetMathLibrary.Normal` _returnvalue_2) (`SceneComponent.GetForwardVector` _vehiclecollision))))
  (set `self.currentMovingDirectionFake` (select `bool` (> _returnvalue 0.0) :`false` (`self.currentHorizontalMovementDirection`) :`true` _returnvalue)))

(fn `HandleFallingTime`
  (params (groundWheelsCount :type Integer))
  (bind _output_get (set `self.isMovingOnGround` (>= groundWheelsCount (`self.minimumGroundedWheelsToMove`))))
  (set `self.fallingTime` (select `bool` _output_get :`false` (+ (`self.fallingTime`) (`self.deltaSeconds`)))))

(fn `HandleSpeedBoost`
  (if (and (`self.isSpeedBoostEnabled`) (`self.isMovingOnGround`) (<= (`self.currentHorizontalSpeed`) (`self.maxBoostSpeed`)))
    (`PrimitiveComponent.AddForce` (`self.VehicleCollision`) (* (`self.GetActorForwardVector`) (* (`self.acceleration`) (`self.speedBoostAccelerationFactor`))) "None" true)))

(fn `InitializeComponentArrays`
  (set `self.wheelMeshList` (`|MakeArray` (`self.FRWheelMesh`) (`self.FLWheelMesh`) (`self.BRWheelMesh`) (`self.BLWheelMesh`)))
  (bind _output_get (set `self.wheelSceneList` (`|MakeArray` (`self.FRWheelScene`) (`self.FLWheelScene`) (`self.BRWheelScene`) (`self.BLWheelScene`))))
  (for _array_element _output_get
    (`KismetArrayLibrary.Array_Add` (`self.localSuspensionPointsList`) (`SceneComponent.RelativeLocation` _array_element))))

(fn `InitializeConfig`
  (if (`self.shouldApplyCustomConfig`)
    (`KismetSystemLibrary.ExecuteConsoleCommand` (`KismetStringLibrary.Concat_StrStr` "t.MaxFPS " (`KismetStringLibrary.Conv_IntToString` (`self.maxFPS`))) (`GameplayStatics.GetPlayerController` 0))))

(fn `InitializeHUD`
  (bind _returnvalue (`|CreateWidget` "/Game/UI/WBP_InGameHUD.WBP_InGameHUD_C" (`GameplayStatics.GetPlayerControllerFromID` (`self.playerID`))))
  (bind _output_get (set `self.inGameHUD` _returnvalue))
  (set `/Game/UI/WBP_InGameHUD.vehicle` self _output_get)
  (`UserWidget.AddToPlayerScreen` _output_get 0))

(fn `InitializePhysicsConfiguration`
  (bind _vehiclecollision (`self.VehicleCollision`))
  (`PrimitiveComponent.SetLinearDamping` _vehiclecollision (`self.linearDamping`))
  (`PrimitiveComponent.SetMassOverrideInKg` _vehiclecollision "None" (`self.massInKg`) true)
  (`PrimitiveComponent.SetAngularDamping` _vehiclecollision (`self.angularDamping`))
  (`PrimitiveComponent.SetCenterOfMass` _vehiclecollision (`self.centerOfMassOffsetWhenFalling`) "None"))

(fn `PerformSuspensionRaycasts`
  (params (suspensionPointWorldLocation :type "Vector Structure") (suspensionPointRelativeLocation :type "Vector Structure"))
  (returns (isGroundHit :type Boolean) (ratio :type "Float (double-precision)") (applyForceLocation :type "Vector Structure"))
  (bind (_returnvalue_x _returnvalue_y _returnvalue_z) (`KismetMathLibrary.BreakVector` (`BoxComponent.GetScaledBoxExtent` (`self.VehicleCollision`))))
  (bind _returnvalue (- suspensionPointWorldLocation (* (`self.GetActorUpVector`) (+ _returnvalue_z (.z suspensionPointRelativeLocation)))))
  (bind (_outhit _returnvalue_2) (`KismetSystemLibrary.SphereTraceSingleForObjects` :`Start` suspensionPointWorldLocation :`End` (- suspensionPointWorldLocation (* (`self.GetActorUpVector`) (`self.suspensionHeight`))) :`Radius` (`self.wheelRadius`) :`ObjectTypes` (`self.walkableObjectTypes`) :`bTraceComplex` (`self.isTraceComplex`) :`DrawDebugType` (select `bool` (`self.isDebugModeEnabled`) :`true` "ForOneFrame" :!type "EDrawDebugTrace Enum")))
  (return _returnvalue_2 (`KismetMathLibrary.FClamp` (`KismetMathLibrary.SelectFloat` (- 1.0 (/ (`KismetMathLibrary.VSize` (- (`.ImpactPoint` (`GameplayStatics.BreakHitResult` _outhit)) _returnvalue)) (`self.suspensionHeight`))) 0.0 _returnvalue_2)) _returnvalue))

(fn `ResetCarCD`
  (set `self.bCanReset` true))

(fn `SetMeshesVisibility`
  (params (visibility :type Boolean))
  (`SceneComponent.SetVisibility` (`self.BodyMesh`) visibility false)
  (`SceneComponent.SetVisibility` (`self.FRWheelMesh`) visibility false)
  (`SceneComponent.SetVisibility` (`self.FLWheelMesh`) visibility false)
  (`SceneComponent.SetVisibility` (`self.BRWheelMesh`) visibility false)
  (`SceneComponent.SetVisibility` (`self.BLWheelMesh`) visibility false))

(fn `SpeedBoostEnd`
  (if (`KismetSystemLibrary.K2_IsTimerActiveHandle` (`self.speedBoostTimerHandle`))
    (`KismetSystemLibrary.K2_ClearAndInvalidateTimerHandle` (`self.speedBoostTimerHandle`)))
  (set `self.isSpeedBoostEnabled` false))

(fn `SpeedBoostStart`
  (params (speedBoostFactor :type "Float (double-precision)" :default 2.0) (autoStop :type Boolean :default true) (speedBoostDuration :type "Float (double-precision)" :default 2.0))
  (set `self.isSpeedBoostEnabled` true)
  (set `self.speedBoostAccelerationFactor` speedBoostFactor)
  (if autoStop
    (bind _returnvalue (`KismetSystemLibrary.K2_SetTimer` null "SpeedBoostEnd" (`KismetMathLibrary.FMax` 0.0 speedBoostDuration)))
    (set `self.speedBoostTimerHandle` _returnvalue)))

(fn `UpdateCenterOfMassOffset`
  (`PrimitiveComponent.SetCenterOfMass` (`self.VehicleCollision`) (select `bool` (> (`self.fallingTime`) 1.0) :`false` (`self.centerOfMassOffsetWhenMoving`) :`true` (`self.centerOfMassOffsetWhenFalling`)) "None"))

(fn `UpdateEngineAudio`
  (`AudioComponent.SetFloatParameter` (`self.EngineAudio`) "Speed" (`self.currentHorizontalSpeed`)))

(fn `UpdateWheelsPosition`
  (for (_array_element _array_index) (`self.wheelSceneList`)
    (bind (_output_x _output_y _output_z) (`KismetMathLibrary.BreakVector` (`|GetArrayItem` (`self.localSuspensionPointsList`) _array_index)))
    (`SceneComponent.K2_SetRelativeLocation` _array_element (`KismetMathLibrary.VLerp` (`SceneComponent.RelativeLocation` _array_element) (`KismetMathLibrary.MakeVector` _output_x _output_y (+ _output_z (* (- 1.0 (`|GetArrayItem` (`self.lastFrameRatios`) _array_index)) (`self.suspensionHeight`) -1.0) (`self.wheelRadius`))) (`KismetMathLibrary.FClamp` (* (`self.deltaSeconds`) 10.0))) false false)))

(fn `UpdateWheelsRotation`
  (for _array_element (`self.wheelMeshList`)
    (`SceneComponent.K2_AddLocalRotation` _array_element (`KismetMathLibrary.MakeRotator` 0.0 (* (`self.currentHorizontalSpeed`) (`self.currentHorizontalMovementDirection`) (`KismetMathLibrary.SignOfFloat` (`KismetMathLibrary.Dot_VectorVector` (`SceneComponent.GetRightVector` _array_element) (`SceneComponent.GetRightVector` (`self.VehicleCollision`)))) (`KismetMathLibrary.GetPI`) (`GameplayStatics.GetWorldDeltaSeconds`) -1.0 0.1)) false false)))

(fn `UpdateWheelsSteering`
  (for _index (range 2)
    (bind _output (`|GetArrayItem` (`self.wheelSceneList`) _index))
    (bind (_relativerotation_roll _relativerotation_pitch _relativerotation_yaw) (`KismetMathLibrary.BreakRotator` (`SceneComponent.RelativeRotation` _output)))
    (`SceneComponent.K2_SetRelativeRotation` _output (`KismetMathLibrary.MakeRotator` 0.0 0.0 (`KismetMathLibrary.Lerp` _relativerotation_yaw (* (`self.GetInputAxisValue`) (`self.maxSteerAngle`)) (* (`self.deltaSeconds`) 15.0))) false false)))

(fn `UseItem`
  (switch `/Game/Blueprints/Gameplay/E_ItemTypes` (`self.currentItemType`)
    (:`NewEnumerator0`
      (`self.SpeedBoostStart` 1.2 true 1.0))
    (:`NewEnumerator1`
      (`self.SpeedBoostStart` 0.8 true 1.0)))
  (set `self.currentItemType` "NewEnumerator2"))

(fn `UserConstructionScript`
  (set `self.lastCheckPointPosition` (`self.GetTransform`))
  (set `self.bCanReset` true))